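; HUD Blueprint that draws a list of named messages, chat-log style, as on-screen text.
; Each DrawHUD call parses the Text string from MyGameInstance as JSON and iterates its "list" array.
; Each entry's nested "m" object supplies "name" and "msg", drawn as a "name:msg" line stacked down the left edge.
; Nothing is drawn when parsing fails, as the raw-text fallback sits inside the success branch.
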(event `self.ReceiveDrawHUD`
  (params (SizeX :type Integer) (SizeY :type Integer))
  (bind _asmy_game_instance (cast `MyGameInstance` (`GameplayStatics.GetGameInstance`)))
  (bind _text (`MyGameInstance.text` _asmy_game_instance))
  (bind (_outjsonobject _returnvalue) (`JsonBlueprintFunctionLibrary.FromString` _text))
  (if _returnvalue
    (bind _outvalue (`|GetJsonField` _outjsonobject "list"))
    (bind _output_get (set `self.jsons` _outvalue))
    (for (_array_element _array_index) _output_get
      (bind _outvalue_2 (`|GetJsonField` _array_element "m"))
      (bind _outvalue_3 (`|GetJsonField` _outvalue_2 "msg"))
      (bind _outvalue_4 (`|GetJsonField` _outvalue_2 "name"))
      (`self.DrawText` (`KismetMathLibrary.SelectString` (`KismetStringLibrary.Concat_StrStr` _outvalue_4 ": " _outvalue_3) _text _returnvalue) (struct :`R` 1.0 :`G` 1.0 :`B` 1.0 :`A` 1.0) 22.0 (`KismetMathLibrary.Conv_IntToDouble` (* _array_index 16)) "/Engine/EngineFonts/DroidSansMono.DroidSansMono"))))

(fn `UserConstructionScript`)